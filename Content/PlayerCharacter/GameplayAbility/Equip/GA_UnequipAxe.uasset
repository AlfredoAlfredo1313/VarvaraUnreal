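; Gameplay ability that unequips the player's axe and stows it on the character's back.
; It plays a disarm montage, clears the equipped weapon tag, and waits for the unequip gameplay event to attach the axe to the spine socket.
; HandleUnequiWeapon then unlinks the axe anim layers, removes its input mapping context and granted abilities, and resets the NeverRelax anim flag.
; The ability ends when the montage completes, blends out or is interrupted.
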(event Ability|EventActivateAbility
  (|PlayMontageandWaitProxy "None" "/Game/PlayerCharacter/Montage/AM_standing_disarm_underarm.AM_standing_disarm_underarm" 1.0 "None" false 1.0 0.0 false
    (:then
      (Variables|/Script/Varvaraa.PawnCombatComponent|SetCurrentEquippedWeaponTag (Class|VarvaraGameplayAbility|GetCombatComponentfromActorInfo) "")
      (Ability|Tasks|WaitGameplayEvent "(TagName=\"Player.Event.UnequipAxe\")" 0
        (:EventReceived
          (Transformation|AttachComponentToComponent (Class|PawnCombatComponent|GetCharacterWeaponfromTag (Class|VarvaraGameplayAbility|GetCombatComponentfromActorInfo) "(TagName=\"Player.Weapon.Axe\")") (Class|GameplayAbility|GetOwningComponentfromActorInfo) "SpineSocket_Axe" "SnapToTarget" "KeepRelative" "KeepWorld" true)
          (CallFunction|HandleUnequiWeapon (Class|VarvaraCombatComponent|GetHeroCarriedWeaponbyTag (Class|VarvaraGameplayAbility|GetCombatComponentfromActorInfo) "(TagName=\"Player.Weapon.Axe\")")))))
    (:OnCompleted
      (Ability|EndAbility :!label _label))
    (:OnBlendOut
      (goto _label))
    (:OnInterrupted
      (goto _label))))

(event Ability|EventOnEndAbility
  (params (bWasCancelled :type Boolean)))

(fn HandleUnequiWeapon
  (params (InWeaponUnequip :type Varvara%20Weapon%20Object%20Reference))
  (LocalVariables|SetWeaponData (Variables|/Script/Varvaraa.VarvaraWeapon|GetHeroWeaponData InWeaponUnequip))
  (Utilities|FlowControl|Sequence
    (:then_0
      (Class|SkeletalMeshComponent|UnlinkAnimClassLayers (Class|GameplayAbility|GetOwningComponentfromActorInfo) (.WeaponAnimLayerToLink (Utilities|Struct|BreakVarvaraWeaponData (Variables|/Script/Varvaraa.VarvaraWeapon|GetHeroWeaponData (Class|VarvaraCombatComponent|GetHeroCarriedWeaponbyTag (Class|VarvaraGameplayAbility|GetCombatComponentfromActorInfo) "(TagName=\"Player.Weapon.Axe\")"))))))
    (:then_1
      (Input|RemoveMappingContext (PlayerController|LocalPlayerSubsystems|GetEnhancedInputLocalPlayerSubsystem (Class|VarvaraGameplayAbility|GetVarvaraControllerfromActorInfo)) "/Game/PlayerCharacter/Input/IMC_Axe.IMC_Axe" "(bIgnoreAllPressedKeysUntilRelease=True,bForceImmediately=False,bNotifyUserSettings=False)")
      (Variables|/Script/Varvaraa.PawnCombatComponent|SetCurrentEquippedWeaponTag (Class|VarvaraGameplayAbility|GetCombatComponentfromActorInfo) "(TagName=\"\")"))
    (:then_2
      (Class|BaseAbilitySystemComponent|RemoveGrantedWeaponAbilities (Class|BaseGameplayAbility|GetBaseAbilitySystemComponentfromActorInfo) (Class|VarvaraWeapon|GetGrantedWeaponAbilities InWeaponUnequip)))
    (:then_3
      (Variables|/Script/Varvaraa.VarvaraAnimInstance|SetbNeverRelax (Class|VarvaraGameplayAbility|GetVarvaraAnimInstancefromActorInfo) false))))